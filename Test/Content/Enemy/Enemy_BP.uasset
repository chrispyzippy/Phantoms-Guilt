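; Enemy character that chases the player on sight and makes a melee attack, and reports itself as targettable.
; PawnSensing sets IsSeeingPlayer and starts an AI MoveTo toward the player, while Tick halts movement whenever the flag is false.
; On arrival it plays the attack montage behind a Delay-based cooldown, or clears the flag if still cooling down.
; A parallel sequence branch adds a single random movement nudge after a short delay.
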(event `self.ReceiveTick`
  (params (DeltaSeconds :type "Float (single-precision)"))
  (if (not (`self.Is_Seeing_Player`))
    (`MovementComponent.StopMovementImmediately` (`self.CharacterMovement`))))

(event `self.PawnSensing.OnSeePawn`
  (params (Pawn :type "Pawn Object Reference"))
  (set `self.Is_Seeing_Player` true)
  (`self.Follow_Player`))

(event `Follow_Player`
  (bind _returnvalue (`KismetMathLibrary.RandomFloat`))
  (if (`self.Is_Seeing_Player`)
    (`|AIMoveTo` self (0.0 0.0 0.0) (`GameplayStatics.GetPlayerCharacter` 0) 150.0
      (:`OnSuccess`
        (`|ExecutionSequence`
          (:`then_0`
            (if (`self.Can_Attack`)
              (set `self.Can_Attack` false)
              (`self.PlayAnimMontage` "/Game/Enemy/Enemy_Anim/Enemy_Attack.Enemy_Attack")
              (`KismetSystemLibrary.Delay` 5.0)
              (set `self.Can_Attack` true)
              (else
                (set `self.Is_Seeing_Player` false))))
          (:`then_1`
            (`KismetSystemLibrary.Delay` 1.0)
            (`self.AddMovementInput` (`KismetMathLibrary.Conv_DoubleToVector` _returnvalue) _returnvalue)
            (`KismetSystemLibrary.Delay` 1.0)))))))

(fn `Targettable `
  (returns (Target :type Boolean))
  (return true))

(fn `UserConstructionScript`)